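; Game instance that acts as the central hub for menus, HUD widgets, pausing and UI audio.
; Show events lazily create and cache each widget before adding it to the viewport, with title and level-select also setting menu state and selectable-item count.
; A pause toggle drives the pause menu, and small events play theme and UI cues.
; RandomSound picks a body-hit cue behind a DoOnce; SaveGameCheck is an empty stub.
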(event Custom|Show%20Title%20Widget
  ;[1 1 1] Show Title Widget
  (Utilities|IsValid (Variables|WB|GetMainMenu_WB)
    (:Is%20Valid
      _)
    (:Is%20Not%20Valid
      (bind _returnvalue (UserInterface|CreateWidget "/Game/widget/Menu_Main.Menu_Main_C" (Game|GetPlayerController 0)))
      (Variables|WB|SetMainMenu_WB _returnvalue)))
  (UserInterface|Viewport|AddtoViewport (Variables|WB|GetMainMenu_WB) 0)
  (CallFunction|SwitchMenu "NewEnumerator0" (Class|PanelWidget|GetChildrenCount (Variables|/Game/widget/Menu_Main.Menu_Main_C|GetMainMenu_Box (Variables|WB|GetMainMenu_WB)))))

(event Custom|Play%20cancel%20Sounnd
  ;[1 1 1] Play sound
  (Audio|PlaySound2D "/Game/Sound/UI/UI_cancel_mst__Cue.UI_cancel_mst__Cue"))

(event Custom|Switch%20Menu
  (params (SwitchMenu :type State%20Enum :default "NewEnumerator0") (MaxSelectChild :type Integer))
  ;[1 1 1] Switch Menu Event
  (Variables|Default|SetCurrentState SwitchMenu)
  (Variables|Default|SetMaxSelectChild MaxSelectChild))

(event Custom|Show%20Count%20Wdiget
  ;[1 1 1] Show Count Widget
  (Utilities|IsValid (Variables|Default|GetCountWidgetWB)
    (:Is%20Valid
      _)
    (:Is%20Not%20Valid
      (bind _returnvalue (UserInterface|CreateWidget "/Game/widget/count.count_C"))
      (Variables|Default|SetCountWidgetWB _returnvalue)))
  (UserInterface|Viewport|AddtoViewport (Variables|Default|GetCountWidgetWB) 0))

(event Custom|Play%20open%20level%20sound
  ;[1 1 1] Play sound
  (Audio|PlaySound2D "/Game/Sound/UI/UI_choosen_3nts_Cue.UI_choosen_3nts_Cue"))

(event Custom|Show_Player_Lose_Widget
  ;[1 1 1] Show Player Lose Widget
  (Utilities|IsValid (Variables|WB|GetPlayer_Lose_WB)
    (:Is%20Valid
      _)
    (:Is%20Not%20Valid
      (bind _returnvalue (UserInterface|CreateWidget "/Game/widget/Player_LOSE.Player_Lose_C" (Game|GetPlayerController 0)))
      (Variables|WB|SetPlayer_Lose_WB _returnvalue)))
  (UserInterface|Viewport|AddtoViewport (Variables|WB|GetPlayer_Lose_WB) 0))

(event Custom|Show%20Level%20Info
  ;[1 1 1] Show level info
  (Utilities|IsValid (Variables|Default|Getlevel%20info%20WB)
    (:Is%20Valid
      _)
    (:Is%20Not%20Valid
      (bind _returnvalue (UserInterface|CreateWidget "/Game/widget/Level_Information.Level_Information_C"))
      (Variables|Default|Setlevel%20info%20WB _returnvalue)))
  (UserInterface|Viewport|AddtoViewport (Variables|Default|Getlevel%20info%20WB) 0))

(event Custom|Play%20MainTheme
  ;[1 1 1] Play sound
  (Audio|PlaySound2D "/Game/Sound/MainTheme_Cue.MainTheme_Cue"))

(event Custom|Pause%20/%20Resume%20Game
  ;[1 1 1] Show pause menu
  (if (Game|IsGamePaused)
    (Game|SetGamePaused false)
    (Widget|RemovefromParent (Variables|Default|GetGamePauseWB))
    (else
      (Game|SetGamePaused true)
      (CallFunction|ShowPauseMenu))))

(event Custom|SaveGameCheck
  ;[1 1 1] save game check
)

(event Custom|Play%20Confirm%20Sound
  ;[1 1 1] Play sound
  (Audio|PlaySound2D "/Game/Sound/UI/UI_choosen_mst_Cue.UI_choosen_mst_Cue"))

(event Custom|Show%20Select%20Level%20Widget
  ;[1 1 1] Show Select Level Widget
  (Utilities|IsValid (Variables|WB|GetSelectLevel_WB)
    (:Is%20Valid
      _)
    (:Is%20Not%20Valid
      (bind _returnvalue (UserInterface|CreateWidget "/Game/widget/Menu_SelectLevel.Menu_SelectLevel_C" (Game|GetPlayerController 0)))
      (Variables|WB|SetSelectLevel_WB _returnvalue)))
  (UserInterface|Viewport|AddtoViewport (Variables|WB|GetSelectLevel_WB) 0)
  (CallFunction|SwitchMenu "NewEnumerator1" (Variables|Default|GetNumber_of_Level)))

(event Custom|Player%20Select%20Sound
  ;[1 1 1] Play sound
  (Audio|PlaySound2D "/Game/Sound/UI/UI_selscted_mst_Cue.UI_selscted_mst_Cue"))

(event Custom|Show_Player_Win_Widget
  ;[1 1 1] Show Player Win Widget
  (Utilities|IsValid (Variables|WB|GetPlayer_Win_WB)
    (:Is%20Valid
      _)
    (:Is%20Not%20Valid
      (bind _returnvalue (UserInterface|CreateWidget "/Game/widget/Player_Win.Player_Win_C" (Game|GetPlayerController 0)))
      (Variables|WB|SetPlayer_Win_WB _returnvalue)))
  (UserInterface|Viewport|AddtoViewport (Variables|WB|GetPlayer_Win_WB) 0))

(event Custom|Show%20Pause%20Menu
  ;[1 1 1] Show Pause Menu Event
  (Utilities|IsValid (Variables|Default|GetGamePauseWB)
    (:Is%20Valid
      _)
    (:Is%20Not%20Valid
      (bind _returnvalue (UserInterface|CreateWidget "/Game/widget/Menu_Game_Pause.Menu_Game_Pause_C"))
      (Variables|Default|SetGamePauseWB _returnvalue)))
  (UserInterface|Viewport|AddtoViewport (Variables|Default|GetGamePauseWB) 0))

(fn RandomSound
  (Variables|Default|Setint (Math|Random|RandomInteger 4))
  (Utilities|FlowControl|DoOnce false
    (:Completed
      (if (== (Variables|Default|Getint) 1)
        (Audio|PlaySoundatLocation "/Game/Sound/Character/BodyHit01Update_Cue.BodyHit01Update_Cue" "0, 0, 0")
        (elif (== (Variables|Default|Getint) 2)
          (Audio|PlaySoundatLocation "/Game/Sound/Character/BodyHit02UpDate_Cue.BodyHit02UpDate_Cue" "0, 0, 0")
          (elif (== (Variables|Default|Getint) 3)
            (Audio|PlaySoundatLocation "/Game/Sound/Character/BodyHit_Moan_HI_Cue.BodyHit_Moan_HI_Cue" "0, 0, 0")
            (elif (== (Variables|Default|Getint) 4)
              (Audio|PlaySoundatLocation "/Game/Sound/Character/BodyHit_Moan_HI_Cue.BodyHit_Moan_HI_Cue" "0, 0, 0")
              (elif (== (Variables|Default|Getint) 5)
                (Audio|PlaySoundatLocation "/Game/Sound/Character/BodyHit_Moan_MID_Cue.BodyHit_Moan_MID_Cue" "0, 0, 0")
                (else
                  (Audio|PlaySoundatLocation "/Game/Sound/Character/BodyHit_MoanLO_Cue.BodyHit_MoanLO_Cue" "0, 0, 0"))))))))))