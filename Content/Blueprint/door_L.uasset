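; Left-hand sliding door panel that opens and closes along world Y, driven by the door state in MyGameState.
; Tick polls the open flag and wait time, steps the actor by a fixed per-frame offset while open, then clears the shared flag after a Delay.
; CloseDoor waits the game state's door time, then enables an opposite Tick-applied offset for a fixed duration, so travel depends on frame rate.
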(event Custom|close%20door
  (Utilities|FlowControl|Delay (Variables|Default|Getdoor%20open%20time))
  (Variables|Default|Setmove2 4.0)
  (Utilities|FlowControl|Delay 1.5)
  (Variables|Default|Setmove2 0.0))

(event EventBeginPlay
  (Variables|Default|Setlocation (Transformation|GetActorLocation)))

(event Collision|EventActorBeginOverlap
  (params (OtherActor :type Actor%20Object%20Reference)))

(event EventTick
  (params (DeltaSeconds :type Float%20%28single-precision%29))
  (Utilities|FlowControl|Sequence
    (:then_0
      (bind _asmy_game_state (Utilities|Casting|CastToMyGameState (Game|GetGameState))
        (:then
          (Variables|Default|Setopen? (Variables|/Game/Blueprint/MyGameState.MyGameState_C|Getdoor_state _asmy_game_state))
          (Variables|Default|Setdoor%20open%20time (Variables|/Game/Blueprint/MyGameState.MyGameState_C|Getdoor%20time _asmy_game_state)))
        (:CastFailed
          (Development|PrintString "game state cast fail"))))
    (:then_1
      (if (Variables|Default|Getopen?)
        (bind _output_get (Variables|Default|Setmove -4.0))
        (Transformation|SetActorLocation (+ (Variables|Default|Getlocation) (Math|Vector|MakeVector 0.0 _output_get 0.0)) false false)
        (Variables|Default|Setlocation (+ (Variables|Default|Getlocation) (Math|Vector|MakeVector 0.0 _output_get 0.0)))
        (Utilities|FlowControl|Delay 1.5)
        (Variables|Default|Setmove 0.0)
        (Variables|/Game/Blueprint/MyGameState.MyGameState_C|Setdoor_state _asmy_game_state false)
        (CallFunction|CloseDoor)))
    (:then_2
      (Transformation|SetActorLocation (+ (Variables|Default|Getlocation) (Math|Vector|MakeVector 0.0 (Variables|Default|Getmove2) 0.0)) false false)
      (Variables|Default|Setlocation (+ (Variables|Default|Getlocation) (Math|Vector|MakeVector 0.0 (Variables|Default|Getmove2) 0.0))))))

(fn ConstructionScript)