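; Huangbox is a pickup-style box actor that destroys itself when the player's myCharacter overlaps its Cube.
; On overlap it prints a debug string, plays an explosion sound and spawns a particle emitter at its location.
; It finds the level_3 actor through GetAllActorsOfClass, increments that actor's Peng10ci counter, and calls its 10ci event when the count reaches ten.
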(event OnComponentBeginOverlap(Cube)
  (params (OverlappedComponent :type Primitive%20Component%20Object%20Reference) (OtherActor :type Actor%20Object%20Reference) (OtherComp :type Primitive%20Component%20Object%20Reference) (OtherBodyIndex :type Integer) (bFromSweep :type Boolean) (SweepResult :type Hit%20Result%20Structure%20%28by%20ref%29))
  (bind _returnvalue (Transformation|GetActorLocation))
  (bind _asmy_character (Utilities|Casting|CastTomyCharacter (Game|GetPlayerCharacter 0)))
  (if (== OtherActor _asmy_character)
    (Development|PrintString "destory")
    (Audio|SpawnSoundatLocation "/Game/Sample/Audio/Explosion01.Explosion01" _returnvalue)
    (Effects|SpawnEmitteratLocation "/Game/Blueprint/P_AnimTrail.P_AnimTrail" _returnvalue)
    (bind _outactors (Actor|GetAllActorsOfClass "/Game/Blueprint/levelcontrol/level_3.level_3_C"))
    (bind _aslevel_3 (Utilities|Casting|CastTolevel_3 (Utilities|Array|Get(acopy) _outactors)))
    (Actor|DestroyActor)
    (Variables|/Game/Blueprint/levelcontrol/level_3.level_3_C|Setpeng10ci _aslevel_3 (+ (Variables|/Game/Blueprint/levelcontrol/level_3.level_3_C|Getpeng10ci _aslevel_3) 1))
    (if (== (Variables|/Game/Blueprint/levelcontrol/level_3.level_3_C|Getpeng10ci _aslevel_3) 10)
      (Default|10ci _aslevel_3))))

(event EventBeginPlay)

(event Collision|EventActorBeginOverlap
  (params (OtherActor :type Actor%20Object%20Reference)))

(event EventTick
  (params (DeltaSeconds :type Float%20%28single-precision%29)))

(fn ConstructionScript)