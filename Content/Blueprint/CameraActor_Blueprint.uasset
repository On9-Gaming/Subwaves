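; Camera actor Blueprint that slides along the Y axis to follow a target position stored in the GameInfoInstance game instance.
; BeginPlay caches the GameInfoInstance reference.
; Each Tick, while not at the target Y, it steps a fixed distance toward it at constant X and zero Z.
; The step ignores delta time, so movement speed depends on frame rate.
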(event EventBeginPlay
  (bind _asgame_info_instance (Utilities|Casting|CastToGameInfoInstance (Game|GetGameInstance)))
  (Variables|Default|SetGameInfoInstance _asgame_info_instance))

(event Collision|EventActorBeginOverlap
  (params (OtherActor :type Actor%20Object%20Reference)))

(event EventTick
  (params (DeltaSeconds :type Float%20%28single-precision%29))
  (if (not (Math|Vector|Equal(Vector) (Math|Vector|MakeVector -443.0 (Variables|/Game/Blueprint/GameInfoInstance.GameInfoInstance_C|GetY (Variables|Default|GetGameInfoInstance)) 0.0) (Transformation|GetActorLocation) 0.0001))
    (if (> (Variables|/Game/Blueprint/GameInfoInstance.GameInfoInstance_C|GetY (Variables|Default|GetGameInfoInstance)) (.Y (Math|Vector|BreakVector (Transformation|GetActorLocation))))
      (Transformation|SetActorLocation (Math|Vector|MakeVector -443.0 (+ (.Y (Math|Vector|BreakVector (Transformation|GetActorLocation))) 1e+01) 0.0) false false)
      (else
        (Transformation|SetActorLocation (Math|Vector|MakeVector -443.0 (- (.Y (Math|Vector|BreakVector (Transformation|GetActorLocation))) 1e+01) 0.0) false false)))))

(fn ConstructionScript)