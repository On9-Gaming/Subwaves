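; Game mode that handles the end-of-match win and lose screens for the player.
; On BeginPlay it caches the game instance and game state, with the game state reference not used further here.
; PlayerWin and playerlose events show the matching widget through the game instance, then switch to UI-only input with a visible cursor.
; Only the win path pauses the game.
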(event Custom|Player%20Win
  (bind _game_info_instance_ref (Variables|Default|Getgame%20info%20instance%20ref))
  ;[1 1 1] Comment
  (Game|SetGamePaused true)
  (Default|ShowPlayerWinWidget _game_info_instance_ref)
  (Input|SetInputModeUIOnly (Game|GetPlayerController 0) (Variables|/Game/Blueprint/GameInfoInstance.GameInfoInstance_C|GetPlayer_Win_WB _game_info_instance_ref) "DoNotLock")
  (Variables|/Script/Engine.PlayerController|SetbShowMouseCursor (Game|GetPlayerController 0) true))

(event Custom|player%20lose
  (bind _game_info_instance_ref (Variables|Default|Getgame%20info%20instance%20ref))
  ;[1 1 1] Comment
  (Default|ShowPlayerLoseWidget _game_info_instance_ref)
  (Input|SetInputModeUIOnly (Game|GetPlayerController 0) (Variables|/Game/Blueprint/GameInfoInstance.GameInfoInstance_C|GetPlayer_Lose_WB _game_info_instance_ref) "DoNotLock")
  (Variables|/Script/Engine.PlayerController|SetbShowMouseCursor (Game|GetPlayerController 0) true))

(event EventBeginPlay
  (Utilities|FlowControl|Sequence
    (:then_0
      (bind _asgame_info_instance (Utilities|Casting|CastToGameInfoInstance (Game|GetGameInstance)))
      (Variables|Default|Setgame%20info%20instance%20ref _asgame_info_instance))
    (:then_1
      (bind _asmy_game_state (Utilities|Casting|CastToMyGameState (Game|GetGameState)))
      (Variables|Default|Setmy%20game%20state%20ref _asmy_game_state))
    (:then_2
      (Utilities|Casting|CastTomyCharacter (Game|GetPlayerCharacter 0)))))

(event EventTick
  (params (DeltaSeconds :type Float%20%28single-precision%29)))

(fn ConstructionScript)