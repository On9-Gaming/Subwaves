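; Level 1 control actor that publishes its level information to the game instance.
; On BeginPlay it caches typed references to the game instance, game mode and game state, though only the game instance reference is used afterwards.
; Every tick it copies LevelInfo into the instance's CurrentLevelInfo while IsActivated is true, and destroys itself otherwise.
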(event EventBeginPlay
  (Utilities|FlowControl|Sequence
    (:then_0
      (bind _asgame_info_instance (Utilities|Casting|CastToGameInfoInstance (Game|GetGameInstance)))
      (Variables|ref|Setgame%20info%20instance%20ref _asgame_info_instance))
    (:then_1
      (bind _asmy_game_mode (Utilities|Casting|CastToMyGameMode (Game|GetGameMode)))
      (Variables|ref|Setmy%20game%20mode%20ref _asmy_game_mode))
    (:then_2
      (bind _asmy_game_state (Utilities|Casting|CastToMyGameState (Game|GetGameState)))
      (Variables|ref|Setmy%20game%20state%20ref _asmy_game_state))))

(event EventTick
  (params (DeltaSeconds :type Float%20%28single-precision%29))
  (if (Variables|Default|GetIs%20Activated?)
    (Variables|/Game/Blueprint/GameInfoInstance.GameInfoInstance_C|Setcurrent%20level%20info (Variables|ref|Getgame%20info%20instance%20ref) (Variables|Default|Getlevel%20info))
    (else
      (Actor|DestroyActor))))

(fn ConstructionScript)