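; Level 2 controller actor that runs a timed hit challenge with win and lose screens.
; While activated, Tick writes the level info to the GameInstance and uses a Delay to lower a countdown about once per second.
; Countdown expiry shows the lose widget once without pausing.
; Each T press adds a hit; reaching ten shows the win widget and pauses.
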(event EventBeginPlay
  (Utilities|FlowControl|Sequence
    (:then_0
      (bind _asgame_info_instance (Utilities|Casting|CastToGameInfoInstance (Game|GetGameInstance)))
      (Variables|Default|SetGame%20info%20instence%20Ref _asgame_info_instance))
    (:then_1
      (bind _asmy_game_mode (Utilities|Casting|CastToMyGameMode (Game|GetGameMode)))
      (Variables|Default|SetMy%20Game%20mode%20ref _asmy_game_mode))
    (:then_2
      (bind _asmy_game_state (Utilities|Casting|CastToMyGameState (Game|GetGameState)))
      (Variables|Default|Setmy%20game%20state%20ref _asmy_game_state))))

(event Collision|EventActorBeginOverlap
  (params (OtherActor :type Actor%20Object%20Reference)))

(event EventTick
  (params (DeltaSeconds :type Float%20%28single-precision%29))
  (bind _returnvalue (Game|GetPlayerController 0))
  (if (Variables|Default|Getis%20activated?)
    (Variables|/Game/Blueprint/GameInfoInstance.GameInfoInstance_C|Setcurrent%20level%20info (Variables|Default|GetGame%20info%20instence%20Ref) (Variables|Default|Getlevel%20info))
    (Utilities|FlowControl|Delay 1.0)
    (Variables|Default|Setcount%20down (- (Variables|Default|Getcount%20down) 1))
    (if (<= (Variables|Default|Getcount%20down) 0)
      (Utilities|FlowControl|DoOnce false
        (:Completed
          (bind _returnvalue_2 (UserInterface|CreateWidget "/Game/widget/Player_LOSE.Player_Lose_C"))
          (UserInterface|Viewport|AddtoPlayerScreen _returnvalue_2)
          (Game|SetGamePaused false)
          (Input|SetInputModeUIOnly _returnvalue _returnvalue_2 "DoNotLock")
          (Variables|/Script/Engine.PlayerController|SetbShowMouseCursor _returnvalue true))))))

(event Input|KeyboardEvents|T
  (params (Key :type Key%20Structure))
  (bind _returnvalue (Game|GetPlayerController 0))
  (:Pressed
    (Variables|Default|SetHit%20count (+ (Variables|Default|GetHit%20count) 1))
    (if (>= (Variables|Default|GetHit%20count) 10)
      (bind _returnvalue_2 (UserInterface|CreateWidget "/Game/widget/Player_Win.Player_Win_C"))
      (UserInterface|Viewport|AddtoPlayerScreen _returnvalue_2)
      (Game|SetGamePaused true)
      (Input|SetInputModeUIOnly _returnvalue _returnvalue_2 "DoNotLock")
      (Variables|/Script/Engine.PlayerController|SetbShowMouseCursor _returnvalue true))))

(fn ConstructionScript)