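; Level 7 control Blueprint that publishes its LevelInfo as the game's current level info while it is activated.
; BeginPlay casts and caches references to the GameInfoInstance, GameMode and GameState, though only the game instance is used afterwards.
; Tick polls IsActivated and, while it is true, writes LevelInfo into the game instance's CurrentLevelInfo every frame.
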(event EventBeginPlay
  ;[0 1 0.06638] begin play
  (Utilities|FlowControl|Sequence
    (:then_0
      (bind _asgame_info_instance (Utilities|Casting|CastToGameInfoInstance (Game|GetGameInstance)))
      (Variables|Default|Setgame%20infro%20instance%20ref _asgame_info_instance))
    (:then_1
      (bind _asgame_mode (Utilities|Casting|CastToGameMode (Game|GetGameMode)))
      (Variables|Default|Setgame%20mode%20ref _asgame_mode))
    (:then_2
      (bind _asgame_state (Utilities|Casting|CastToGameState (Game|GetGameState)))
      (Variables|Default|Setgame%20state%20ref _asgame_state))))

(event Collision|EventActorBeginOverlap
  (params (OtherActor :type Actor%20Object%20Reference)))

(event EventTick
  (params (DeltaSeconds :type Float%20%28single-precision%29))
  (if (Variables|Default|Getis%20activated?)
    (Variables|/Game/Blueprint/GameInfoInstance.GameInfoInstance_C|Setcurrent%20level%20info (Variables|Default|Getgame%20infro%20instance%20ref) (Variables|Default|Getlevel%20info))))

(fn ConstructionScript)