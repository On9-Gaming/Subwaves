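; Level 3 control actor that runs a timed challenge, showing win or lose widgets through the game instance.
; BeginPlay caches game instance, mode and state, then shows the lose screen after ten seconds unless a success flag is set.
; While activated, it publishes its level info every Tick, and key 6 spawns a Cityzen near the player, sets that flag and shows the win screen after a delay.
; The win-collision overlap handler only prints debug text.
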(event Custom|OnActorBeginOverlap_事件_collisionToWin
  (params (OverlappedActor :type Actor%20Object%20Reference) (OtherActor :type Actor%20Object%20Reference))
  (EventDispatchers|AssignOnActorBeginOverlap (delegate Custom|OnActorBeginOverlap_事件_collisionToWin))
  (Development|PrintString "rrrrr"))

(event EventBeginPlay
  ;[0 1 0.06638] begin play
  (Utilities|FlowControl|Sequence
    (:then_0
      (bind _asgame_info_instance (Utilities|Casting|CastToGameInfoInstance (Game|GetGameInstance)))
      (Variables|Default|Setgame%20infro%20instance%20ref _asgame_info_instance))
    (:then_1
      (bind _asgame_mode (Utilities|Casting|CastToGameMode (Game|GetGameMode)))
      (Variables|Default|Setgame%20mode%20ref _asgame_mode))
    (:then_2
      (bind _asgame_state (Utilities|Casting|CastToGameState (Game|GetGameState)))
      (Variables|Default|Setgame%20state%20ref _asgame_state))
    (:then_3
      (Utilities|FlowControl|Delay 1e+01)
      (if (not (Variables|Default|Get10s))
        (Default|ShowPlayerLoseWidget (Variables|Default|Getgame%20infro%20instance%20ref))))))

(event Collision|EventActorBeginOverlap
  (params (OtherActor :type Actor%20Object%20Reference)))

(event EventTick
  (params (DeltaSeconds :type Float%20%28single-precision%29))
  (if (Variables|Default|Getis%20activated?)
    (Variables|/Game/Blueprint/GameInfoInstance.GameInfoInstance_C|Setcurrent%20level%20info (Variables|Default|Getgame%20infro%20instance%20ref) (Variables|Default|Getlevel%20info))))

(event Input|KeyboardEvents|6
  (params (Key :type Key%20Structure))
  (:Pressed
    (if (Variables|Default|Getis%20activated?)
      (Game|SpawnActorfromClass "/Game/AI/cityzen.cityzen_C" (Math|Conversions|ToTransform(Vector) (+ (Transformation|GetActorLocation (Game|GetPlayerCharacter 0)) "0,6.000000,100.000000")) "Undefined" 0 0)
      (Variables|Default|Set10s true)
      (Utilities|FlowControl|Delay 2.0)
      (Default|ShowPlayerWinWidget (Variables|Default|Getgame%20infro%20instance%20ref)))))

(fn ConstructionScript)