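; Subway Blueprint that toggles a Moving flag for a train, with Q calling MOVE and E calling STOP.
; Subway1's begin overlap also calls STOP unless its OverlappedComponent equals the first Plane actor found, comparing its own component rather than the other actor.
; The Moving check and fixed Y-offset SetActorLocation are unwired, and Tick and railway axis events are empty, so this graph never moves the actor.
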(event OnComponentBeginOverlap(subway1)
  (params (OverlappedComponent :type Primitive%20Component%20Object%20Reference) (OtherActor :type Actor%20Object%20Reference) (OtherComp :type Primitive%20Component%20Object%20Reference) (OtherBodyIndex :type Integer) (bFromSweep :type Boolean) (SweepResult :type Hit%20Result%20Structure%20%28by%20ref%29))
  (bind _outactors (Actor|GetAllActorsOfClass "/Game/Blueprint/plane.plane_C"))
  (if (not (== OverlappedComponent (Utilities|Array|Get(acopy) _outactors)))
    (CallFunction|STOP)))

(event Custom|MOVE
  (Variables|Default|Setmoving? true))

(event Custom|STOP
  (Variables|Default|Setmoving? false))

(event EventBeginPlay)

(event EventTick
  (params (DeltaSeconds :type Float%20%28single-precision%29)))

(event Input|AxisEvents|InputAxisrailwaymove
  (params (AxisValue :type Float%20%28single-precision%29)))

(event Input|AxisEvents|InputAxisrailwayback
  (params (AxisValue :type Float%20%28single-precision%29)))

(event Input|KeyboardEvents|Q
  (params (Key :type Key%20Structure :default "AnyKey"))
  (:Pressed
    (CallFunction|MOVE)))

(event Input|KeyboardEvents|E
  (params (Key :type Key%20Structure :default "AnyKey"))
  (:Pressed
    (CallFunction|STOP)))

(fn ConstructionScript)