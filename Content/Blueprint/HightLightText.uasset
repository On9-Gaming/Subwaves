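; Menu navigation controller that moves a highlighted text selection in the main menu and level select screens using input actions.
; A delayed Tick pulls widget references from GameInfoInstance and enables up/down or left/right input based on its current state.
; Direction presses change CurrentSelect, re-highlight the active widget and play a sound.
; Start/Pause confirms through that widget, and Back reopens the title level after a short delay.
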(event Custom|FlashingSelectedText
  (params (NewParam :type Float%20%28single-precision%29))
  ;[1 0.1722 0.04246] Flashing Selected text
  (Utilities|IsValid (Variables|Default|GetGameInfoInstance)))

(event Custom|Unlock%20Input
  ;[1 1 1] Unlock Input depend on which state is player staying
  (Variables|Default|SetAllow%20Navigation%20U/D false)
  (Variables|Default|SetAllow%20Navigation%20L/R false)
  (switch Utilities|FlowControl|Switch|SwitchonState (Variables|/Game/Blueprint/GameInfoInstance.GameInfoInstance_C|GetCurrentState (Variables|Default|GetGameInfoInstance))
    (:NewEnumerator0
      (Variables|Default|SetAllow%20Navigation%20U/D true))
    (:NewEnumerator1
      (Variables|Default|SetAllow%20Navigation%20L/R true))))

(event Custom|Highlight_Selected_Menu_TEXT
  ;[1 1 1] Switch Menu
  (switch Utilities|FlowControl|Switch|SwitchonState (Variables|/Game/Blueprint/GameInfoInstance.GameInfoInstance_C|GetCurrentState (Variables|Default|GetGameInfoInstance))
    (:NewEnumerator0
      (Utilities|IsValid (Variables|Default|GetMainMenuWB)
        (:Is%20Valid
          (Variables|Default|SetAllow%20Navigation%20U/D true)
          (Default|SelectedTextFunction (Variables|Default|GetMainMenuWB) (Variables|Default|GetCurrent_Select)))))
    (:NewEnumerator1
      (Utilities|IsValid (Variables|Default|GetSelect%20Level%20WB)
        (:Is%20Valid
          (Variables|Default|SetAllow%20Navigation%20L/R true)
          (Default|SelectedTextFunction (Variables|Default|GetSelect%20Level%20WB) (Variables|Default|GetCurrent_Select)))))))

(event EventBeginPlay
  ;[0.4135 1 0.4468] event begin play
  (bind _asgame_info_instance (Utilities|Casting|CastToGameInfoInstance (Game|GetGameInstance)))
  (Variables|Default|SetGameInfoInstance _asgame_info_instance)
  (CallFunction|HighlightSelectedMenuTEXT))

(event EventTick
  (params (DeltaSeconds :type Float%20%28single-precision%29))
  (bind _gameinfoinstance (Variables|Default|GetGameInfoInstance))
  ;[1 0.8137 0.2266] Event Tick
  (Utilities|FlowControl|Delay 0.2)
  (Utilities|IsValid (Variables|Default|GetGameInfoInstance)
    (:Is%20Valid
      (CallFunction|UnlockInput)
      (Utilities|FlowControl|Sequence
        (:then_0
          (Variables|Default|SetMainMenuWB (Variables|/Game/Blueprint/GameInfoInstance.GameInfoInstance_C|GetMainMenu_WB _gameinfoinstance)))
        (:then_1
          (Variables|Default|SetSelect%20Level%20WB (Variables|/Game/Blueprint/GameInfoInstance.GameInfoInstance_C|GetSelectLevel_WB _gameinfoinstance)))))))

(event Input|ActionEvents|InputActionButtonn_Left
  (params (Key :type Key%20Structure))
  ;[1 1 1] Button Left Event
  (:Pressed
    (if (Variables|Default|GetAllow%20Navigation%20L/R)
      (if (>= (+ (Variables|Default|GetCurrent_Select) 1) 0)
        (Variables|Default|SetCurrent_Select (- (Variables|Default|GetCurrent_Select) 1))
        (CallFunction|HighlightSelectedMenuTEXT)
        (Default|PlayerSelectSound (Variables|Default|GetGameInfoInstance))))))

(event Input|ActionEvents|InputActionBack
  (params (Key :type Key%20Structure))
  ;[1 1 1] Comment
  (:Pressed
    (Default|PlayCancelSounnd (Variables|Default|GetGameInfoInstance))
    (Utilities|FlowControl|Delay 0.3)
    (Game|OpenLevel(byName) "title")))

(event Input|ActionEvents|InputActionStart/Pause
  (params (Key :type Key%20Structure))
  ;[1 1 1] Press Start button
  (:Pressed
    (switch Utilities|FlowControl|Switch|SwitchonState (Variables|/Game/Blueprint/GameInfoInstance.GameInfoInstance_C|GetCurrentState (Variables|Default|GetGameInfoInstance))
      (:NewEnumerator0
        (Utilities|IsValid (Variables|Default|GetMainMenuWB)
          (:Is%20Valid
            (Default|PressEnter (Variables|Default|GetMainMenuWB) (Variables|Default|GetCurrent_Select))
            (Default|PlayConfirmSound (Variables|Default|GetGameInfoInstance)))))
      (:NewEnumerator1
        (Utilities|IsValid (Variables|Default|GetSelect%20Level%20WB)
          (:Is%20Valid
            (Default|PressEnter (Variables|Default|GetSelect%20Level%20WB))
            (Default|PlayOpenLevelSound (Variables|Default|GetGameInfoInstance))))))))

(event Input|ActionEvents|InputActionButton_Up
  (params (Key :type Key%20Structure))
  ;[1 1 1] Button Up Event
  (:Pressed
    (if (Variables|Default|GetAllow%20Navigation%20U/D)
      (if (>= (- (Variables|Default|GetCurrent_Select) 1) 0)
        (Variables|Default|SetCurrent_Select (- (Variables|Default|GetCurrent_Select) 1))
        (CallFunction|HighlightSelectedMenuTEXT)
        (Default|PlayerSelectSound (Variables|Default|GetGameInfoInstance))))))

(event Input|ActionEvents|InputActionButton_Down
  (params (Key :type Key%20Structure))
  ;[1 1 1] Button Down Event
  (:Pressed
    (if (Variables|Default|GetAllow%20Navigation%20U/D)
      (if (<= (+ (Variables|Default|GetCurrent_Select) 1) (- (Variables|/Game/Blueprint/GameInfoInstance.GameInfoInstance_C|GetMaxSelectChild (Variables|Default|GetGameInfoInstance)) 1))
        (Variables|Default|SetCurrent_Select (+ (Variables|Default|GetCurrent_Select) 1))
        (CallFunction|HighlightSelectedMenuTEXT)
        (Default|PlayerSelectSound (Variables|Default|GetGameInfoInstance))))))

(event Input|ActionEvents|InputActionButton_Right
  (params (Key :type Key%20Structure))
  ;[1 1 1] Buton Right Event
  (:Pressed
    (if (Variables|Default|GetAllow%20Navigation%20L/R)
      (if (<= (+ (Variables|Default|GetCurrent_Select) 1) (- (Variables|/Game/Blueprint/GameInfoInstance.GameInfoInstance_C|GetMaxSelectChild (Variables|Default|GetGameInfoInstance)) 1))
        (Variables|Default|SetCurrent_Select (+ (Variables|Default|GetCurrent_Select) 1))
        (CallFunction|HighlightSelectedMenuTEXT)
        (Default|PlayerSelectSound (Variables|Default|GetGameInfoInstance))))))

(fn ConstructionScript)