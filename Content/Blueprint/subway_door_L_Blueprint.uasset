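; Blueprint for a left subway door that plays its opening animation and shares its state through MyGameState.
; On BeginPlay it caches the game state, registers itself as LeftDoor, and copies NewDoorState, which it then polls every Tick into LeftDoorState.
; LEFTdooropen acts only while NewDoorState is false, setting it true and playing the non-looping skeletal mesh animation, with no closing logic.
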(event Custom|LEFT%20door%20open
  (if (not (Variables|/Game/Blueprint/MyGameState.MyGameState_C|Getnew_door_state (Variables|Default|Getsaved%20game%20state)))
    (Variables|/Game/Blueprint/MyGameState.MyGameState_C|Setnew_door_state (Variables|Default|Getsaved%20game%20state) true)
    (Components|Animation|PlayAnimation (Variables|SkeletalMeshActor|GetSkeletalMeshComponent) "/Game/animation/subway_LEFT_door_Anim.subway_LEFT_door_Anim" false)))

(event Custom|check%20left%20door%20state
  (Variables|Default|Setleft%20door%20state (Variables|/Game/Blueprint/MyGameState.MyGameState_C|Getnew_door_state (Variables|Default|Getsaved%20game%20state))))

(event EventBeginPlay
  (bind _asmy_game_state (Utilities|Casting|CastToMyGameState (Game|GetGameState)))
  (bind _output_get (Variables|Default|Setsaved%20game%20state _asmy_game_state))
  (Variables|/Game/Blueprint/MyGameState.MyGameState_C|Setleft%20door _output_get self)
  (Variables|Default|Setleft%20door%20state (Variables|/Game/Blueprint/MyGameState.MyGameState_C|Getnew_door_state _asmy_game_state)))

(event Collision|EventActorBeginOverlap
  (params (OtherActor :type Actor%20Object%20Reference)))

(event EventTick
  (params (DeltaSeconds :type Float%20%28single-precision%29))
  (CallFunction|CheckLeftDoorState))

(fn ConstructionScript)